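; Actor component that selects combat actions from a DataTable and triggers their montages through a dispatcher, with input buffering and cancels.
; BeginPlay caches table rows by command and ID, and lookups also match the owner's airborne state, judged by upward velocity.
; SaveAction and CheckActionCancel test commands against bitmasks of allowed actions.
; ActionCancel plays the matching entry from a cancel list, either directly by ID or by command, then clears cancel state.
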(event `self.ReceiveBeginPlay`
  (bind _dt_actionlist (`self.DT_ActionList`))
  (`/Engine/EditorBlueprintResources/StandardMacros.IsValid` _dt_actionlist
    (:`Is Valid`
      (bind _outrownames (`DataTableFunctionLibrary.GetDataTableRowNames` _dt_actionlist))
      (for _array_element _outrownames
        (bind _returnvalue (`|GetDataTableRow` _dt_actionlist _array_element)
          (:`then`
            (bind (_actioncommand _damage _canuseinair _montage) (break `/Game/Blueprints/Struct/ST_Action` _returnvalue))
            (`KismetArrayLibrary.Array_Add` (`self.ActionList`) (make `/Game/Blueprints/Struct/ST_Action` _actioncommand _damage _canuseinair _montage (`KismetStringLibrary.Conv_NameToString` _array_element)))))))
    (:`Is Not Valid`
      (`KismetSystemLibrary.PrintString` "Error : DT_Action List가 꽂히지 않았습니다."))))

(fn `ActionCancel`
  (params (`Action Command` :type "/Game/PC/Common/Enum_ActionCommand Enum" :default "NewEnumerator0"))
  (locals (AC_ActionCommand :type "/Game/PC/Common/Enum_ActionCommand Enum") (AC_ActionId :type String) (AC_ForceExecute :type Boolean))
  (for _array_element (`self.ActionCancelList`)
    (if (`|EnumEquality` `Action Command` (break `/Game/Blueprints/Struct/ST_ActionCancel` _array_element))
      (set `local.AC_ActionCommand` (break `/Game/Blueprints/Struct/ST_ActionCancel` _array_element))
      (set `local.AC_ActionId` (`.ActionId_24_44C765A641B2B0C120FF9E8180736001` (break `/Game/Blueprints/Struct/ST_ActionCancel` _array_element)))
      (set `local.AC_ForceExecute` (`.ForceExecute_26_E633351E4FBB26362F92B5B403D90C2E` (break `/Game/Blueprints/Struct/ST_ActionCancel` _array_element)))
      (break)))
  (`self.ClearActionCancel`)
  (if (`local.AC_ForceExecute`)
    (`self.PlayAction_Execute` (`local.AC_ActionId`))
    (else
      (`self.PlayAction` (`local.AC_ActionCommand`) (`local.AC_ActionId`)))))

(fn `Add Action Cancel List`
  (params (`Action Command` :type "/Game/PC/Common/Enum_ActionCommand Enum" :default "NewEnumerator0") (`Action Id` :type String) (`Force Execute` :type Boolean))
  (`KismetArrayLibrary.Array_Add` (`self.ActionCancelList`) (make `/Game/Blueprints/Struct/ST_ActionCancel` `Action Command` `Action Id` `Force Execute`)))

(fn `Check Action Cancel`
  (params (`Action Command` :type "/Game/PC/Common/Enum_ActionCommand Enum" :default "NewEnumerator0") (`Action Id` :type String))
  (returns (Bool :type Boolean))
  (locals (Result :type Boolean))
  (set `local.Result` (> (`KismetMathLibrary.And_IntInt` (`self.Can Action Cancel`) (`KismetMathLibrary.FTrunc` (`KismetMathLibrary.MultiplyMultiply_FloatFloat` 2.0 (`KismetMathLibrary.Conv_IntToDouble` (`KismetMathLibrary.Conv_ByteToInt` `Action Command`))))) 0))
  (return (`local.Result`)))

(fn `ClearActionCancel`
  (set `self.Is Save Action?` false)
  (set `self.Save Action Id` "")
  (set `self.ANS_ActionCancel` false)
  (`KismetArrayLibrary.Array_Clear` (`self.ActionCancelList`)))

(fn `ClearSaveAction`
  (set `self.Is Save Action?` false)
  (set `self.Save Action Id` ""))

(fn `GetSaveAction`
  (returns (`Action Command` :type "/Game/PC/Common/Enum_ActionCommand Enum") (`Action Id` :type String) (`Is Save Action` :type Boolean))
  (if (`self.Is Save Action?`)
    (return (`self.Save Action Command`) (`self.Save Action Id`) (`self.Is Save Action?`))
    (else
      (`KismetSystemLibrary.PrintString` "Error : Not have Save Action")
      (return "NewEnumerator0" "" false))))

(fn `IsInAir`
  (params (CheckActor :type "Actor Object Reference"))
  (returns (Return :type Boolean))
  (bind (_returnvalue_x _returnvalue_y _returnvalue_z) (`KismetMathLibrary.BreakVector` (`CharacterMovementComponent.GetLastUpdateVelocity` (`Actor.GetComponentByClass` CheckActor "/Script/Engine.CharacterMovementComponent"))))
  (return (> _returnvalue_z 0.1)))

(fn `PlayAction`
  (params (`Action Command` :type "/Game/PC/Common/Enum_ActionCommand Enum" :default "NewEnumerator0") (`Action Id` :type String))
  (for _array_element (`self.ActionList`)
    (if (`|EnumEquality` `Action Command` (break `/Game/Blueprints/Struct/ST_Action` _array_element))
      (bind _return (`self.IsInAir` (`self.GetOwner`)))
      (if (== _return (`.CanUseInAir_28_8898ED6F438EC7F029CC60ACC0375AF8` (break `/Game/Blueprints/Struct/ST_Action` _array_element)))
        (if (`KismetStringLibrary.NotEqual_StrStr` `Action Id`)
          (if (`KismetStringLibrary.EqualEqual_StrStr` `Action Id` (`.ActionId_24_44C765A641B2B0C120FF9E8180736001` (break `/Game/Blueprints/Struct/ST_Action` _array_element)))
            (`self.PlayMontage` (`.Montage_32_27B8518443C4E6C8B3FC6F9664596321` (break `/Game/Blueprints/Struct/ST_Action` _array_element)) (`.ActionId_24_44C765A641B2B0C120FF9E8180736001` (break `/Game/Blueprints/Struct/ST_Action` _array_element)))
            (break))
          (else
            (`self.PlayMontage` (`.Montage_32_27B8518443C4E6C8B3FC6F9664596321` (break `/Game/Blueprints/Struct/ST_Action` _array_element)) (`.ActionId_24_44C765A641B2B0C120FF9E8180736001` (break `/Game/Blueprints/Struct/ST_Action` _array_element)))
            (break)))))))

(fn `PlayAction_Execute`
  (params (`Action Id` :type String))
  (for _array_element (`self.ActionList`)
    (if (`KismetStringLibrary.NotEqual_StrStr` `Action Id`)
      (bind _return (`self.IsInAir` (`self.GetOwner`)))
      (if (== _return (`.CanUseInAir_28_8898ED6F438EC7F029CC60ACC0375AF8` (break `/Game/Blueprints/Struct/ST_Action` _array_element)))
        (if (`KismetStringLibrary.EqualEqual_StrStr` `Action Id` (`.ActionId_24_44C765A641B2B0C120FF9E8180736001` (break `/Game/Blueprints/Struct/ST_Action` _array_element)))
          (`self.PlayMontage` (`.Montage_32_27B8518443C4E6C8B3FC6F9664596321` (break `/Game/Blueprints/Struct/ST_Action` _array_element)) (`.ActionId_24_44C765A641B2B0C120FF9E8180736001` (break `/Game/Blueprints/Struct/ST_Action` _array_element)))
          (break)))
      (else
        (`KismetSystemLibrary.PrintString` "PlayAction_Execute Error : No Action Id!")))))

(fn `SaveAction`
  (params (`Action Command` :type "/Game/PC/Common/Enum_ActionCommand Enum" :default "NewEnumerator0") (`Action Id` :type String))
  (if (> (`KismetMathLibrary.And_IntInt` (`self.Can Save Action`) (`KismetMathLibrary.FTrunc` (`KismetMathLibrary.MultiplyMultiply_FloatFloat` 2.0 (`KismetMathLibrary.Conv_IntToDouble` (`KismetMathLibrary.Conv_ByteToInt` `Action Command`))))) 0)
    (set `self.Is Save Action?` true)
    (set `self.Save Action Command` `Action Command`)
    (set `self.Save Action Id` `Action Id`)))