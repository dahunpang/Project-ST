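; Input buffer component that detects multi-input command sequences and returns the matching action name.
; BeginPlay loads command patterns from DTCommandList, while AddInput keeps a capped, timestamped buffer, merging rapid repeats of one input.
; CheckCommandMatch scans the buffer newest to oldest, allowing limited stray inputs within per-step grace times, picks the longest match and clears the buffer.
; MaxDuration is carried but never checked, and IsLimitedFuzzyMatch is an unused stub.
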(event `self.ReceiveBeginPlay`
  (`self.InitCommandParttern`))

(fn `AddInput`
  (params (`FInput Command` :type "/Game/Blueprints/Struct/ST_FInputCommand Structure"))
  (returns (`Input Buffer` :type "Array of /Game/Blueprints/Struct/ST_FInputCommand Structure"))
  (locals (CurrentTime :type "Float (double-precision)") (MinInputInterval :type "Float (double-precision)" :default 0.03))
  (bind _inputbuffer (`self.InputBuffer`))
  (bind _inputbuffer_2 (`self.InputBuffer`))
  (bind _last_input_type (`self.Last Input Type`))
  (set `local.CurrentTime` (`KismetSystemLibrary.GetGameTimeInSeconds`))
  (if (and (`|EnumEquality` _last_input_type `FInput Command_Input_2_F73928E5429B2B88A5F3808242F05381`) (< (- (`local.CurrentTime`) (`self.Last Input Time`)) (`local.MinInputInterval`)))
    (`KismetArrayLibrary.Array_Set` _inputbuffer_2 (- (`KismetArrayLibrary.Array_Length` _inputbuffer_2) 1) (make `/Game/Blueprints/Struct/ST_FInputCommand` _last_input_type (`local.CurrentTime`)))
    (set `self.Last Input Time` (`local.CurrentTime`))
    (else
      (`KismetArrayLibrary.Array_Add` _inputbuffer (make `/Game/Blueprints/Struct/ST_FInputCommand` `FInput Command_Input_2_F73928E5429B2B88A5F3808242F05381` (`KismetSystemLibrary.GetGameTimeInSeconds`)))
      (if (> (`KismetArrayLibrary.Array_Length` _inputbuffer) (`self.BufferMaxSize`))
        ;[0.15 0.15 0.15 0.5 12] 0번을 지우면 자동으로 시프트 된다
        (`KismetArrayLibrary.Array_Remove` _inputbuffer))
      (set `self.Last Input Type` `FInput Command_Input_2_F73928E5429B2B88A5F3808242F05381`)
      (set `self.Last Input Time` (`local.CurrentTime`))
      (return (`self.InputBuffer`)))))

(fn `CheckCommandMatch`
  (params (InputBuffer :type "Array of /Game/Blueprints/Struct/ST_FInputCommand Structure"))
  (returns (`Action Id` :type "/Game/PC/Common/Enum_ActionCommand Enum"))
  (locals (j :type Integer) (i :type Integer) (LastMatchedTime :type "Float (double-precision)") (Return :type Boolean) (iskipCount :type Integer) (LastTimeStamp :type "Float (double-precision)") (`Command Index` :type Integer))
  (bind _bestcommandpattern_actionname (break `/Game/Blueprints/Struct/ST_FCommandPattern` (`self.BestCommandPattern`)))
  (set `self.BestMatchLegnth` -1)
  (for _array_element (`self.CommandPatterns`)
    (bind (_ismatchfound _command_longest) (`self.IsLimitedFuzzyMatch_0` (`.Sequence_3_037BCF1A4E59E88AC32D45B7C8471234` (break `/Game/Blueprints/Struct/ST_FCommandPattern` _array_element)) (`.MaxDuration_8_3E80D28C4E0D02EE47E34E8661984690` (break `/Game/Blueprints/Struct/ST_FCommandPattern` _array_element)) (`.GraceTimeperStep_10_4783CA5C4361A80F791F83B08E2BE7C7` (break `/Game/Blueprints/Struct/ST_FCommandPattern` _array_element)) InputBuffer))
    (if _ismatchfound
      (set `self.MatchFound` _ismatchfound)
      (if (> _command_longest (`self.BestMatchLegnth`))
        (set `self.BestMatchLegnth` _command_longest)
        (set `self.BestCommandPattern` (make `/Game/Blueprints/Struct/ST_FCommandPattern` (break `/Game/Blueprints/Struct/ST_FCommandPattern` _array_element) (`.Sequence_3_037BCF1A4E59E88AC32D45B7C8471234` (break `/Game/Blueprints/Struct/ST_FCommandPattern` _array_element)) (`.MaxDuration_8_3E80D28C4E0D02EE47E34E8661984690` (break `/Game/Blueprints/Struct/ST_FCommandPattern` _array_element)) (`.GraceTimeperStep_10_4783CA5C4361A80F791F83B08E2BE7C7` (break `/Game/Blueprints/Struct/ST_FCommandPattern` _array_element)))))))
  (if (`self.MatchFound`)
    (`self.ClearBuffer`)
    (return _bestcommandpattern_actionname)))

(fn `ClearBuffer`
  (`KismetArrayLibrary.Array_Clear` (`self.InputBuffer`))
  (set `self.BestMatchLegnth` 0))

(fn `Get Save Input Action`
  (returns (`Is Save` :type Boolean))
  (return (`self.Is Save`)))

(fn `InitCommandParttern`
  (bind _dt_commandlist (`self.DT_CommandList`))
  (`/Engine/EditorBlueprintResources/StandardMacros.IsValid` _dt_commandlist
    (:`Is Valid`
      (bind _outrownames (`DataTableFunctionLibrary.GetDataTableRowNames` _dt_commandlist))
      (for _array_element _outrownames
        (bind _returnvalue (`|GetDataTableRow` _dt_commandlist _array_element)
          (:`then`
            (bind (_actionname _sequence _maxduration _gracetimeperstep) (break `/Game/Blueprints/Struct/ST_FCommandPattern` _returnvalue))
            (`KismetArrayLibrary.Array_Add` (`self.CommandPatterns`) (make `/Game/Blueprints/Struct/ST_FCommandPattern` _actionname _sequence _maxduration _gracetimeperstep))))))))

(fn `IsLimitedFuzzyMatch`
  (params (InputBuffer :type "Array of /Game/Blueprints/Struct/ST_FInputCommand Structure") (CommandSequence :type "Array of /Game/PC/Common/Enum_InputType Enum") (`Max Duration` :type "Float (double-precision)") (`Grace Timeper Step` :type "Float (double-precision)") (bufferlength :type Integer))
  (returns (IsMatchFound :type Boolean) (`Command Longest` :type Integer))
  (locals (i :type Integer) (j :type Integer) (iskipCount :type Integer) (CommandIndex :type Integer) (return :type Boolean) (`Match Found` :type Boolean) (LastTimeStamp :type "Float (double-precision)")))

(fn `IsLimitedFuzzyMatch_0`
  (params (CommandSequence :type "Array of /Game/PC/Common/Enum_InputType Enum") (`Max Duration` :type "Float (double-precision)") (`Grace Timeper Step` :type "Float (double-precision)") (`Input Buffer` :type "Array of /Game/Blueprints/Struct/ST_FInputCommand Structure"))
  (returns (IsMatchFound :type Boolean) (`Command Longest` :type Integer))
  (locals (i :type Integer) (j :type Integer) (iskipCount :type Integer) (CommandIndex :type Integer) (return :type Boolean) (`Match Found` :type Boolean) (LastTimeStamp :type "Float (double-precision)"))
  (set `local.LastTimeStamp` (`KismetSystemLibrary.GetGameTimeInSeconds`))
  (set `local.Match Found` false)
  (set `local.return` false)
  (set `local.iskipCount` 0)
  (set `local.CommandIndex` (`KismetArrayLibrary.Array_Length` CommandSequence))
  (bind (_arrayindex _arrayelement) (`/Engine/EditorBlueprintResources/StandardMacros.ReverseForEachLoop` `Input Buffer`)
    (:`LoopBody`
      (if (!= (`local.return`) true)
        ; 입력 텀이 커맨드 텀보다 길면 안됨
        (if (< (- (`local.LastTimeStamp`) (`.TimeStamp_5_50A55DB5431139BEABF79ABA80297CA5` (break `/Game/Blueprints/Struct/ST_FInputCommand` _arrayelement))) `Grace Timeper Step`)
          (set `local.LastTimeStamp` (`.TimeStamp_5_50A55DB5431139BEABF79ABA80297CA5` (break `/Game/Blueprints/Struct/ST_FInputCommand` _arrayelement)))
          (if (`|EnumEquality` (break `/Game/Blueprints/Struct/ST_FInputCommand` _arrayelement) (`|GetArrayItem` CommandSequence (- (`local.CommandIndex`) 1)))
            (bind _output_get (set `local.CommandIndex` (- (`local.CommandIndex`) 1)))
            (if (<= _output_get 0)
              (set `local.Match Found` true)
              (set `local.return` true))
            (else
              (set `local.iskipCount` (+ (`local.iskipCount`) 1))
              (if (> (`local.iskipCount`) (`self.MaxSkipButton`))
                (set `local.Match Found` false)
                (set `local.return` true)))))))
    (:`Completed`
      (set `local.return` false)
      (set `local.iskipCount` 0)
      (return (`local.Match Found`) (`KismetArrayLibrary.Array_Length` CommandSequence)))))