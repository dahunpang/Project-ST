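; BP_Hero is a hero character Blueprint in the legacy Hero_Riven folder that sets an initial action state and displays it for debugging.
; On BeginPlay it calls the parent, then switches its action component to the Character.Base.Idle gameplay tag.
; Every Tick it reads the current action and draws that tag as a debug string on itself.
; The overlap event is disabled, and the construction script only calls its parent.
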(event `self.ReceiveBeginPlay`
  (`parent.ReceiveBeginPlay`)
  (`self.ChangeActionTag` self (`self.액션 컴포넌트`) (struct :`TagName` "Character.Base.Idle")))

(event `self.ReceiveTick`
  (params (DeltaSeconds :type "Float (single-precision)"))
  (`parent.ReceiveTick` DeltaSeconds)
  (bind _action (`self.Get Current Action` false))
  (`KismetSystemLibrary.DrawDebugString` (0.0 0.0 0.0) (`BlueprintGameplayTagLibrary.GetDebugStringFromGameplayTag` _action) self))

(fn `UserConstructionScript`
  (`parent.UserConstructionScript`))