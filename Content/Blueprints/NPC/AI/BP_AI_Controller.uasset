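; AI controller for NPCs that runs the BT_NPC_NORMAL behavior tree and feeds it player-detection data through the Blackboard.
; AI perception flags sensed "Player"-tagged actors as the enemy and enables per-tick distance updates, which are never switched off.
; Other perception updates start a timer that, on expiry, saves the character's location and clears line of sight, enemy and attack stance.
; A new sighting cancels that timer.
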(event `self.ReceiveTick`
  (params (DeltaSeconds :type "Float (single-precision)"))
  ;[1 1 1] NPC (자신)와 PC(적)의 거리를 측정함 → DistanceToEnemyActor (블랙보드 키)에 거리 값 전달
  (if (`self.PlayerCheck`)
    (`BlackboardComponent.SetValueAsFloat` (`self.Blackboard`) (`self.DistanceToEnemyActor`) (`self.GetDistanceTo` (`self.FindPawn`) (`self.IsPlayer?`)))))

(event `self.ReceivePossess`
  (params (PossessedPawn :type "Pawn Object Reference"))
  (set `self.FindPawn` PossessedPawn)
  (`self.RunBehaviorTree` "/Game/Blueprints/NPC/BT/BT_NPC_NORMAL.BT_NPC_NORMAL"))

(event `self.AIPerception.OnTargetPerceptionUpdated`
  (params (Actor :type "Actor Object Reference") (Stimulus :type "AIStimulus Structure"))
  (if (and (`self.ActorHasTag` Actor "Player") (`.bSuccessfullySensed` (break `AIStimulus` Stimulus)))
    (set `self.IsPlayer?` Actor)
    (`KismetSystemLibrary.K2_ClearAndInvalidateTimerHandle` (`self.Enemy Timer`))
    (`BlackboardComponent.SetValueAsBool` (`self.Blackboard`) (`self.Has Line Of Sight`) true)
    (`BlackboardComponent.SetValueAsObject` (`self.Blackboard`) (`self.Enemy Actor`) Actor)
    (`BlackboardComponent.SetValueAsBool` (`self.Blackboard`) (`self.DidFindEnemy`) true)
    (`|ExecutionSequence`
      (:`then_0`
        (set `self.PlayerCheck` true)))
    (else
      (bind _returnvalue (`KismetSystemLibrary.K2_SetTimerDelegate` (delegate `StartEnemyTimer`) (`self.Line Of Sight Timer`)))
      (set `self.Enemy Timer` _returnvalue))))

(event `StartEnemyTimer`
  (bind _asbp_character (cast `/Game/Blueprints/Legacy/PC/Common/BP_Character` (stale `self.AIPerception.OnTargetPerceptionUpdated` Actor)))
  (`BlackboardComponent.SetValueAsVector` (`self.Blackboard`) (`self.EnemyActorLastLocation`) (`self.K2_GetActorLocation` _asbp_character))
  (`BlackboardComponent.SetValueAsBool` (`self.Blackboard`) (`self.Has Line Of Sight`) false)
  (`BlackboardComponent.SetValueAsObject` (`self.Blackboard`) (`self.Enemy Actor`) null)
  (`BlackboardComponent.SetValueAsBool` (`self.Blackboard`) (`self.SetStanceAttack`) false))

(fn `UserConstructionScript`)