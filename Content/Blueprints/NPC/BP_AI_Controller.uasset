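; AI controller for an NPC that runs the BT_NPC_BOSS behavior tree on possess and tracks sight of the player.
; When perception senses a Player-tagged actor, it sets HasLineOfSight and EnemyActor on the blackboard and cancels any pending forget timer.
; Any other perception update starts a LineOfSightTimer delay, after which both keys are cleared.
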(event `self.ReceivePossess`
  (params (PossessedPawn :type "Pawn Object Reference"))
  (`self.RunBehaviorTree` "/Game/Blueprints/NPC/BT_NPC_BOSS.BT_NPC_BOSS"))

(event `self.AIPerception.OnTargetPerceptionUpdated`
  (params (Actor :type "Actor Object Reference") (Stimulus :type "AIStimulus Structure"))
  (if (and (`self.ActorHasTag` Actor "Player") (`.bSuccessfullySensed` (break `AIStimulus` Stimulus)))
    (`KismetSystemLibrary.K2_ClearAndInvalidateTimerHandle` (`self.Enemy Timer`))
    (`BlackboardComponent.SetValueAsBool` (`self.Blackboard`) (`self.Has Line Of Sight`) true)
    (`BlackboardComponent.SetValueAsObject` (`self.Blackboard`) (`self.Enemy Actor`) Actor)
    (else
      (bind _returnvalue (`KismetSystemLibrary.K2_SetTimerDelegate` (delegate `StartEnemyTimer`) (`self.Line Of Sight Timer`)))
      (set `self.Enemy Timer` _returnvalue))))

(event `StartEnemyTimer`
  (bind _blackboard (`self.Blackboard`))
  (`BlackboardComponent.SetValueAsBool` _blackboard (`self.Has Line Of Sight`) false)
  (`BlackboardComponent.SetValueAsObject` _blackboard (`self.Enemy Actor`) null))

(fn `UserConstructionScript`)