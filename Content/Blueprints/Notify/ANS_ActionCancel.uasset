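; ANS_ActionCancel is an animation notify state that cancels into a saved action on the owner's BPC_ActionComponent.
; When the notify begins with an action saved, it looks up that action's command in its ActionCancel list to get an ActionId.
; It passes both to PlayAction and clears the saved action, even if no entry matched.
; The saved action is checked only at notify begin, as the tick does nothing.
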(fn `Action Check`
  (params (`Input Action Command` :type "/Game/PC/Common/Enum_ActionCommand Enum" :default "NewEnumerator0"))
  (returns (`Action Id` :type String))
  (locals (`Final Action Id` :type String))
  (for _array_element (`self.Action Cancel`)
    (if (`|EnumEquality` `Input Action Command` (break `/Game/Blueprints/Struct/ST_ActionCancel` _array_element))
      (set `local.Final Action Id` (`.ActionId_24_44C765A641B2B0C120FF9E8180736001` (break `/Game/Blueprints/Struct/ST_ActionCancel` _array_element)))
      (break)))
  (return (`local.Final Action Id`)))

(fn `Received_NotifyBegin`
  (params (MeshComp :type "SkeletalMeshComponent Object Reference") (Animation :type "AnimSequenceBase Object Reference") (TotalDuration :type "Float (single-precision)") (EventReference :type "AnimNotifyEventReference Structure (by ref)"))
  (returns (ReturnValue :type Boolean))
  (bind _returnvalue (`Actor.GetComponentByClass` (`ActorComponent.GetOwner` MeshComp) "/Game/Blueprints/Component/BPC_ActionComponent.BPC_ActionComponent_C"))
  (if (`/Game/Blueprints/Component/BPC_ActionComponent.Is Save Action?` _returnvalue)
    (bind _action_command (`/Game/Blueprints/Component/BPC_ActionComponent.GetSaveAction` _returnvalue))
    (bind _action_id (`self.Action Check` _action_command))
    (`/Game/Blueprints/Component/BPC_ActionComponent.PlayAction` _returnvalue _action_command _action_id)
    (`/Game/Blueprints/Component/BPC_ActionComponent.ClearSaveAction` _returnvalue)
    (return false)))

(fn `Received_NotifyTick`
  (params (MeshComp :type "SkeletalMeshComponent Object Reference") (Animation :type "AnimSequenceBase Object Reference") (FrameDeltaTime :type "Float (single-precision)") (EventReference :type "AnimNotifyEventReference Structure (by ref)"))
  (returns (ReturnValue :type Boolean))
  (return false))