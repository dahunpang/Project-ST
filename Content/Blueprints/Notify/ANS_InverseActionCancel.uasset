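; Animation notify state that flags an inverse action cancel window on the owning actor's BPC_ActionComponent.
; On begin it sets ANSInverseActionCancel to true and copies its CanSaveActionCommand value into the component's CanSaveAction.
; On end it clears only ANSInverseActionCancel, leaving CanSaveAction as set.
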(fn `Received_NotifyBegin`
  (params (MeshComp :type "SkeletalMeshComponent Object Reference") (Animation :type "AnimSequenceBase Object Reference") (TotalDuration :type "Float (single-precision)") (EventReference :type "AnimNotifyEventReference Structure (by ref)"))
  (returns (ReturnValue :type Boolean))
  (bind _returnvalue (`Actor.GetComponentByClass` (`ActorComponent.GetOwner` MeshComp) "/Game/Blueprints/Component/BPC_ActionComponent.BPC_ActionComponent_C"))
  (set `/Game/Blueprints/Component/BPC_ActionComponent.ANS_InverseActionCancel` true _returnvalue)
  (set `/Game/Blueprints/Component/BPC_ActionComponent.Can Save Action` (`self.Can Save Action Command`) _returnvalue)
  (return false))

(fn `Received_NotifyEnd`
  (params (MeshComp :type "SkeletalMeshComponent Object Reference") (Animation :type "AnimSequenceBase Object Reference") (EventReference :type "AnimNotifyEventReference Structure (by ref)"))
  (returns (ReturnValue :type Boolean))
  (set `/Game/Blueprints/Component/BPC_ActionComponent.ANS_InverseActionCancel` false (`Actor.GetComponentByClass` (`ActorComponent.GetOwner` MeshComp) "/Game/Blueprints/Component/BPC_ActionComponent.BPC_ActionComponent_C"))
  (return false))