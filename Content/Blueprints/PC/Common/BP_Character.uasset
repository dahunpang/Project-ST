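; Player character Blueprint with camera-relative movement, hold-Space lock-on and a gameplay-tag action system.
; BeginPlay maps the action component's entries by tag, and ChangeActionTag uses that map to set the current action and play its montage.
; Key-triggered action commands record press or release input for combo transitions.
; Movement input requires the Walk tag, and Tick rotates the moving character toward the locked NPC or input direction.
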(event `self.ReceiveBeginPlay`
  (`self.Initializer ActionTag` (`self.액션 컴포넌트`))
  (`/Game/Blueprints/PC/Common/LockonComp.SetLockOnCamera` (`self.LockonPosition`) (`self.SpringArm`)))

(event `Key|SpaceBar` :consume false
  (params (Key :type "Key Structure"))
  (:`Pressed`
    (bind _enemy (`self.FindEnemy` null "/Game/Blueprints/NPC/BP_Class/BP_Npc_Parant.BP_Npc_Parant_C"))
    (`/Game/Blueprints/PC/Common/LockonComp.SetLockOn` (`self.LockonPosition`) _enemy)
    (set `self.LockOn` true)
    (set `self.LockTarget` _enemy))
  (:`Released`
    (`/Game/Blueprints/PC/Common/LockonComp.SetLockOff` (`self.LockonPosition`))
    (set `self.LockOn` false)))

(event `InputAxis|Turn`
  (params (AxisValue :type "Float (single-precision)"))
  (`SceneComponent.K2_AddRelativeRotation` (`self.SpringArm`) (`KismetMathLibrary.MakeRotator` 0.0 0.0 (* AxisValue 0.3)) false false))

(event `InputAxis|LookUp`
  (params (AxisValue :type "Float (single-precision)"))
  (`SceneComponent.K2_AddRelativeRotation` (`self.SpringArm`) (`KismetMathLibrary.MakeRotator` 0.0 (* AxisValue -0.3)) false false))

(event `InputAxis|MoveForward` :consume false
  (params (AxisValue :type "Float (single-precision)"))
  (if (== (`self.CurrentAction`) (struct :`TagName` "Character.Base.Walk"))
    (bind _output_get (set `self.MoveX` AxisValue))
    (`self.AddMovementInput` (`SceneComponent.GetForwardVector` (`self.Camera`)) _output_get)))

(event `InputAxis|MoveRight` :consume false
  (params (AxisValue :type "Float (single-precision)"))
  (if (== (`self.CurrentAction`) (struct :`TagName` "Character.Base.Walk"))
    (bind _output_get (set `self.MoveY` AxisValue))
    (`self.AddMovementInput` (`SceneComponent.GetRightVector` (`self.Camera`)) _output_get)))

(event `self.ReceiveTick`
  (params (DeltaSeconds :type "Float (single-precision)"))
  (bind _returnvalue (`self.K2_GetActorLocation`))
  (bind (_returnvalue_roll _returnvalue_pitch _returnvalue_yaw) (`KismetMathLibrary.BreakRotator` (`self.K2_GetActorRotation`)))
  (bind _returnvalue_2 (`self.K2_GetActorLocation` (`self.LockTarget`)))
  (bind (_returnvalue_roll_2 _returnvalue_pitch_2 _returnvalue_yaw_2) (`KismetMathLibrary.BreakRotator` (`KismetMathLibrary.Conv_VectorToRotator` (+ (* (`SceneComponent.GetForwardVector` (`self.Camera`)) (`KismetMathLibrary.SignOfFloat` (`self.MoveX`))) (* (`SceneComponent.GetRightVector` (`self.Camera`)) (`KismetMathLibrary.SignOfFloat` (`self.MoveY`)))))))
  (bind _bool (`self.IsMoveable`))
  (set `self.IsAddMovement` _bool)
  (if _bool
    (`|ExecutionSequence`
      (:`then_1`
        (if (`self.IsAddMovement`)
          (if (`self.LockOn`)
            (`self.K2_SetActorRotation` (`KismetMathLibrary.RInterpTo` (`self.K2_GetActorRotation`) (`KismetMathLibrary.FindLookAtRotation` _returnvalue _returnvalue_2) (`GameplayStatics.GetWorldDeltaSeconds`) 35.0))
            (set `self.LockOnTargetVector` (`KismetMathLibrary.Normal` (- _returnvalue_2 _returnvalue)))
            (else
              (`self.K2_SetActorRotation` (`KismetMathLibrary.RInterpTo` (`KismetMathLibrary.MakeRotator` 0.0 0.0 _returnvalue_yaw) (`KismetMathLibrary.MakeRotator` 0.0 0.0 _returnvalue_yaw_2) (`GameplayStatics.GetWorldDeltaSeconds`) 34.0)))))))
    (elif (and (== (`self.CurrentAction`) (struct :`TagName` "Character.Base.Walk")) (== (`KismetMathLibrary.VSize` (`self.GetVelocity`)) 0.0))
      (set `self.CurrentAction` (struct :`TagName` "Character.Base.Idle")))))

(fn `ChangeActionTag`
  (params (`Action Comp` :type "/Game/Blueprints/PC/Common/ActionComponent Object Reference") (`Action Id` :type "GameplayTag Structure"))
  (bind _returnvalue (`SkeletalMeshComponent.GetAnimInstance` (`self.GetComponentByClass` (`ActorComponent.GetOwner` `Action Comp`) "/Script/Engine.SkeletalMeshComponent")))
  (bind _actiontag (`self.GetActionTag` `Action Id` `Action Comp`))
  (bind _output_get (set `self.CurrentAction` (break `/Game/Blueprints/PC/Common/S_ActionTag` _actiontag)))
  (if (`KismetSystemLibrary.IsValid` (`.ActionMontage_6_59D27BA24F4D50865CE3BC8D44F14DD5` (break `/Game/Blueprints/PC/Common/S_ActionTag` _actiontag)))
    (`/Engine/EditorBlueprintResources/StandardMacros.IsValid` _returnvalue
      (:`Is Valid`
        (`AnimInstance.Montage_Play` _returnvalue (`.ActionMontage_6_59D27BA24F4D50865CE3BC8D44F14DD5` (break `/Game/Blueprints/PC/Common/S_ActionTag` _actiontag)) 1.0 "MontageLength" 0.0 true)))
    (elif (not (== _output_get (struct :`TagName` "Character.Base.Walk")))
      (`KismetSystemLibrary.PrintString` "해당 액션 태그에 몽타주가 설정되어 있지 않습니다!")
      (`KismetSystemLibrary.PrintString` (`BlueprintGameplayTagLibrary.GetDebugStringFromGameplayTag` (break `/Game/Blueprints/PC/Common/S_ActionTag` _actiontag)))
      (`KismetSystemLibrary.PrintString` (`KismetSystemLibrary.GetObjectName` (`ActorComponent.GetOwner` `Action Comp`))))))

(fn `CleanActionCommand`
  (params (RemoveAll :type Boolean) (pressKey :type "Key Structure" :default "None"))
  (bind _actioncommand (`self.ActionCommand`))
  (if RemoveAll
    (`KismetArrayLibrary.Array_Clear` _actioncommand)
    (`KismetArrayLibrary.Array_Resize` _actioncommand)
    (else
      (for (_array_element _array_index) (`self.ActionCommand`)
        (if (== pressKey (break `/Game/Blueprints/PC/Common/S_ActionCommand` _array_element))
          (`KismetArrayLibrary.Array_Remove` (`self.ActionCommand`) _array_index))))))

(fn `FindEnemy`
  (params (rootActor :type "Actor Object Reference") (FindEnemyClass :type "Actor Class Reference"))
  (returns (Enemy :type "Actor Object Reference"))
  (locals (closeEnemyDistance :type "Float (double-precision)" :default 15000.0) (lockOnTarget :type "Actor Object Reference"))
  (bind _outactors (`GameplayStatics.GetAllActorsOfClass` FindEnemyClass))
  (for _array_element _outactors
    (bind _returnvalue (`self.GetDistanceTo` _array_element rootActor))
    (if (< _returnvalue (`local.closeEnemyDistance`))
      (set `local.closeEnemyDistance` _returnvalue)
      (set `local.lockOnTarget` _array_element)))
  (`/Engine/EditorBlueprintResources/StandardMacros.IsValid` (`local.lockOnTarget`)
    (:`Is Valid`
      (`KismetSystemLibrary.PrintString` "찾음")
      (return (`local.lockOnTarget`)))
    (:`Is Not Valid`
      (`KismetSystemLibrary.PrintString` "못찾음"))))

(fn `Get Current Action`
  (params (`Get Previous Action?` :type Boolean))
  (returns (Action :type "GameplayTag Structure"))
  (if `Get Previous Action?`
    (return (`self.PreviousAction`))
    (else
      (return (`self.CurrentAction`)))))

(fn `GetActionCommand`
  (params (PressKey :type "Key Structure" :default "None"))
  (returns (ActionCommand :type "/Game/Blueprints/PC/Common/S_ActionCommand Structure"))
  (if (> (`KismetArrayLibrary.Array_Length` (`self.ActionCommand`)) 0)
    (for _array_element (`self.ActionCommand`)
      (if (== PressKey (`.PressKey_3_501F54C546168E865BAA88BE984FFA70` (break `/Game/Blueprints/PC/Common/S_ActionCommand` _array_element)))
        (return _array_element)))
    (else
      (`KismetSystemLibrary.PrintString` "가져올 수 있는 ActionCommand가 없습니다!"))))

(fn `GetActionTag`
  (params (`Action Id` :type "GameplayTag Structure") (`Action Comp` :type "/Game/Blueprints/PC/Common/ActionComponent Object Reference"))
  (returns (ActionTag :type "/Game/Blueprints/PC/Common/S_ActionTag Structure"))
  (bind (_value _returnvalue) (`BlueprintMapLibrary.Map_Find` (`/Game/Blueprints/PC/Common/ActionComponent.Actioncontainer` (`self.액션 컴포넌트`)) `Action Id`))
  (if (not _returnvalue)
    (`KismetSystemLibrary.PrintString` (`KismetStringLibrary.Concat_StrStr` "해당 캐릭터가 사용할 수 없는 액션입니다." (`BlueprintGameplayTagLibrary.GetDebugStringFromGameplayTag` `Action Id`)) _returnvalue))
  (return _value))

(fn `Initializer ActionTag`
  (params (Actor :type "/Game/Blueprints/PC/Common/ActionComponent Object Reference (by ref)"))
  (bind _actioncontainer (`/Game/Blueprints/PC/Common/ActionComponent.Actioncontainer` (`self.액션 컴포넌트`)))
  (bind _actiontag (`/Game/Blueprints/PC/Common/ActionComponent.ActionTag` (`self.액션 컴포넌트`)))
  (if (> (`KismetArrayLibrary.Array_Length` _actiontag) 0)
    (for _array_element _actiontag
      (`BlueprintMapLibrary.Map_Add` _actioncontainer (`.ActionId_2_86F4DA574ACC32D1C2C7AD8FBC9FA3F3` (break `/Game/Blueprints/PC/Common/S_ActionTag` _array_element)) _array_element))
    (`KismetSystemLibrary.PrintString` (`KismetStringLibrary.Concat_StrStr` "ActionContainer 설정 완료 총 개수 : " (`KismetStringLibrary.Conv_IntToString` (`BlueprintMapLibrary.Map_Length` _actioncontainer))))))

(fn `IsEnableActionCommand`
  (returns (bool :type Boolean))
  (return (> (`KismetArrayLibrary.Array_Length` (`self.ActionCommand`)) 0)))

(fn `IsMoveable`
  (returns (bool :type Boolean))
  (return (> (+ (`KismetMathLibrary.Abs` (`self.MoveX`)) (`KismetMathLibrary.Abs` (`self.MoveY`))) 0.0)))

(fn `Set Current Action`
  (params (Action :type "GameplayTag Structure") (Montage :type "AnimMontage Object Reference"))
  (bind _output_get (set `self.CurrentAction` Action))
  (set `self.PreviousAction` _output_get)
  (`AnimInstance.Montage_Play` (`SkeletalMeshComponent.GetAnimInstance` (`self.Mesh`)) Montage 1.0 "MontageLength" 0.0 true))

(fn `Set FirstAction Tag`
  (params (ActionTag :type "GameplayTag Structure"))
  (`self.Set Current Action` ActionTag))

(fn `SetActionCommand`
  (params (PressKey :type "Key Structure" :default "None") (ChangeAcitonTag :type "GameplayTag Structure") (PressType :type "/Game/Blueprints/PC/Common/E_PressAndRelease Enum" :default "NewEnumerator0"))
  (`KismetArrayLibrary.Array_Add` (`self.ActionCommand`) (make `/Game/Blueprints/PC/Common/S_ActionCommand` PressKey PressType false ChangeAcitonTag)))

(fn `SetCanbePressKey`
  (params (bool :type Boolean))
  (set `self.CanbePressKey` bool))

(fn `UserConstructionScript`)

(fn `WhenKeyPressed`
  (params (PressKey :type "Key Structure" :default "None"))
  ;[1 1 1] 액션도중 조작시
  (if (> (`KismetArrayLibrary.Array_Length` (`self.ActionCommand`)) 0)
    (for (_array_element _array_index) (`self.ActionCommand`)
      (if (== (break `/Game/Blueprints/PC/Common/S_ActionCommand` _array_element) PressKey)
        (`KismetArrayLibrary.Array_Set` (`self.ActionCommand`) _array_index (make `/Game/Blueprints/PC/Common/S_ActionCommand` (break `/Game/Blueprints/PC/Common/S_ActionCommand` _array_element) (`.TriggerType_25_CCD992C6465BFE4BF578CAA5EEEF6C94` (break `/Game/Blueprints/PC/Common/S_ActionCommand` _array_element)) (`|EnumEquality` (`.TriggerType_25_CCD992C6465BFE4BF578CAA5EEEF6C94` (break `/Game/Blueprints/PC/Common/S_ActionCommand` _array_element)) "NewEnumerator0") (`.ComboActionTag_22_BE779E10457A9511B20DDDBCFA85BB96` (break `/Game/Blueprints/PC/Common/S_ActionCommand` _array_element))))))))

(fn `WhenKeyReleased`
  (params (PressKey :type "Key Structure" :default "None"))
  ;[1 1 1] 액션도중 조작시
  (if (> (`KismetArrayLibrary.Array_Length` (`self.ActionCommand`)) 0)
    (for (_array_element _array_index) (`self.ActionCommand`)
      (if (== (break `/Game/Blueprints/PC/Common/S_ActionCommand` _array_element) PressKey)
        (if (`|EnumEquality` (`.TriggerType_25_CCD992C6465BFE4BF578CAA5EEEF6C94` (break `/Game/Blueprints/PC/Common/S_ActionCommand` _array_element)) "NewEnumerator1")
          (`KismetSystemLibrary.PrintString` "fhewqaoifwheifloweahfilew")
          (`KismetArrayLibrary.Array_Set` (`self.ActionCommand`) _array_index (make `/Game/Blueprints/PC/Common/S_ActionCommand` (break `/Game/Blueprints/PC/Common/S_ActionCommand` _array_element) "NewEnumerator1" true (`.ComboActionTag_22_BE779E10457A9511B20DDDBCFA85BB96` (break `/Game/Blueprints/PC/Common/S_ActionCommand` _array_element)))))))))