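; Lock-on camera component that frames its owner and a target actor by driving a supplied spring arm.
; While locked on, Tick steers the arm toward their midpoint, turns the child camera to face it, and zooms by their on-screen separation.
; After lock-off, a delay precedes easing the arm back to the component's location and disabling tick.
; Moves and resets interpolate through self-rescheduling, frame-length timers.
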(event `self.ReceiveTick`
  (params (DeltaSeconds :type "Float (single-precision)"))
  (if (`self.PressLockon`)
    (`|ExecutionSequence`
      (:`then_0`
        (`/Engine/EditorBlueprintResources/StandardMacros.IsValid` (`self.ClosedActor`)
          (:`Is Valid`
            (bind (_bool _distance) (`self.Is Pawn in Screen` 0.55))
            (if _bool
              ;[1 1 1] 화면 안에 있으나 가까우면 카메라를 떨어뜨림
              (if (and (< _distance 0.25) (> (`Actor.GetDistanceTo` (`self.GetOwner`) (`self.ClosedActor`)) 300.0))
                (bind _asspring_arm_component (cast `SpringArmComponent` (`self.Camera`)))
                (bind _targetarmlength (`SpringArmComponent.TargetArmLength` _asspring_arm_component))
                (set `SpringArmComponent.TargetArmLength` (`KismetMathLibrary.FInterpTo` _targetarmlength (+ _targetarmlength (* (`self.Arm Speed`) -1.0)) (`GameplayStatics.GetWorldDeltaSeconds`) 5.0) _asspring_arm_component))
              (else
                ;[1 1 1] 화면 밖에 있어서 카메라를 줌아웃 함
                (bind _asspring_arm_component_2 (cast `SpringArmComponent` (`self.Camera`)))
                (bind _targetarmlength_2 (`SpringArmComponent.TargetArmLength` _asspring_arm_component_2))
                (set `SpringArmComponent.TargetArmLength` (`KismetMathLibrary.FInterpTo` _targetarmlength_2 (+ _targetarmlength_2 (`self.Arm Speed`)) (`GameplayStatics.GetWorldDeltaSeconds`) 5.0) _asspring_arm_component_2))))))
      (:`then_1`
        (`self.UpdateLockOnLocation`)))
    (else
      ;[1 1 1] 카메라 복구 시간 경과 시 (waitForReturn)
      (if (> (`self.returnSec`) (`self.waitForReturn`))
        (`self.ReSetCameraStart`)
        (`self.SetComponentTickEnabled` false)
        (else
          (set `self.returnSec` (+ (`self.returnSec`) (`GameplayStatics.GetWorldDeltaSeconds`))))))))

(event `ReSetCameraStart`
  (bind _returnvalue (`KismetSystemLibrary.K2_SetTimer` null "ResetCamera" (`GameplayStatics.GetWorldDeltaSeconds`))))

(event `CameraMoveStart`
  (bind _returnvalue (`KismetSystemLibrary.K2_SetTimer` null "CameraMove" (`GameplayStatics.GetWorldDeltaSeconds`)))
  (set `self.CameraTimer` _returnvalue))

(event `self.ReceiveBeginPlay`
  (`self.SetComponentTickEnabled` false))

(event `ReSetCameraEnd`
  (`KismetSystemLibrary.K2_ClearAndInvalidateTimerHandle` (stale `ReSetCameraStart` _returnvalue))
  (set `self.cameraResetDeltaTime` 0.0))

(event `CameraMoveEnd`
  (`KismetSystemLibrary.K2_ClearAndInvalidateTimerHandle` (`self.CameraTimer`)))

(fn `CameraMove`
  (`self.K2_SetWorldLocation` (`self.Camera`) (`KismetMathLibrary.VInterpTo` (`self.K2_GetComponentLocation` (`self.Camera`)) (`self.CameraMoveLocation`) (`GameplayStatics.GetWorldDeltaSeconds`) (`self.Camera Interp Speed`)) false false)
  (if (< (`KismetMathLibrary.Vector_Distance` (`self.K2_GetComponentLocation` (`self.Camera`)) (`self.CameraMoveLocation`)) 23.0)
    (`self.CameraMoveEnd`)
    (else
      (`self.CameraMoveStart`))))

(fn `Is Pawn in Screen`
  (params (CheckDistance :type "Float (double-precision)"))
  (returns (bool :type Boolean) (Distance :type "Float (double-precision)"))
  (bind _closedactor (`self.ClosedActor`))
  (bind _returnvalue (`KismetMathLibrary.Distance2D` (`self.GetActorScreenLocation2D` (`self.GetOwner`)) (`self.GetActorScreenLocation2D` _closedactor)))
  (`/Engine/EditorBlueprintResources/StandardMacros.IsValid` _closedactor
    (:`Is Valid`
      (return (< _returnvalue (`KismetMathLibrary.FClamp` CheckDistance 0.0 1.212)) _returnvalue))
    (:`Is Not Valid`
      (return false 0.0))))

(fn `IsLockOn`
  (returns (bool :type Boolean))
  (return (`self.PressLockon`)))

(fn `ResetCamera`
  (bind _returnvalue (`self.GetOwner`))
  (if (`self.PressLockon`)
    (`self.ReSetCameraEnd`)
    (else
      (`self.CameraMoveEnd`)
      (`self.K2_SetWorldLocation` (`self.Camera`) (`KismetMathLibrary.VInterpTo` (`self.K2_GetComponentLocation` (`self.Camera`)) (`self.K2_GetComponentLocation`) (+ (`self.cameraResetDeltaTime`) (`GameplayStatics.GetWorldDeltaSeconds`)) 5.0) false false)
      (if (< (`KismetMathLibrary.Vector_Distance` (`self.K2_GetComponentLocation` (`self.Camera`)) (`self.K2_GetComponentLocation`)) (`self.InterpDistance`))
        (`/Engine/EditorBlueprintResources/StandardMacros.IsValid` _returnvalue
          (:`Is Valid`
            (cast `/Game/Blueprints/PC/BP_Character` _returnvalue)
            (`self.ReSetCameraEnd`)))
        (else
          (`self.ReSetCameraStart`)
          (set `self.cameraResetDeltaTime` (+ (`self.cameraResetDeltaTime`) (`GameplayStatics.GetWorldDeltaSeconds`))))))))

(fn `SetCameraMove`
  (params (Location :type "Vector Structure") (`Interp Speed` :type "Float (double-precision)"))
  (set `self.CameraMoveLocation` Location)
  (set `self.Camera Interp Speed` `Interp Speed`)
  (if (`KismetSystemLibrary.K2_IsTimerActiveHandle` (`self.CameraTimer`))
    (`self.CameraMoveStart`)
    (else
      (`self.CameraMoveStart`))))

(fn `SetLockOff`
  (set `self.PressLockon` false)
  (set `self.returnSec` 0.0))

(fn `SetLockOn`
  (params (Actor :type "Actor Object Reference"))
  (set `self.PressLockon` true)
  (`/Engine/EditorBlueprintResources/StandardMacros.IsValid` Actor
    (:`Is Valid`
      (bind _output_get (set `self.ClosedActor` Actor))
      (`self.SetCameraMove` (`self.GetMidPoint` (`self.K2_GetComponentLocation` (`self.Camera`)) (`Actor.K2_GetActorLocation` _output_get)) 15.0)
      (`self.SetComponentTickEnabled` true))))

(fn `SetLockOnCamera`
  (params (SpringArm :type "SceneComponent Object Reference"))
  (set `self.Camera` SpringArm))

(fn `UpdateLockOnLocation`
  (bind _mid_point_location (`self.GetMidPoint` (`Actor.K2_GetActorLocation` (`self.GetOwner` self)) (`Actor.K2_GetActorLocation` (`self.ClosedActor`))))
  (`/Engine/EditorBlueprintResources/StandardMacros.IsValid` (`self.ClosedActor`)
    (:`Is Valid`
      (set `self.CameraMoveLocation` _mid_point_location)
      (set `self.Camera Interp Speed` 3.5)
      (bind `_as카메라_컴포넌트` (cast `CameraComponent` (`self.GetChildComponent` (`self.Camera`) 0)))
      (`self.K2_SetWorldRotation` `_as카메라_컴포넌트` (`KismetMathLibrary.RInterpTo` (`SceneComponent.RelativeRotation` (`self.Camera`)) (`KismetMathLibrary.FindLookAtRotation` (`self.K2_GetComponentLocation` `_as카메라_컴포넌트`) _mid_point_location) (`GameplayStatics.GetWorldDeltaSeconds`) 2.5) false false)
      (if (not (`KismetSystemLibrary.K2_IsValidTimerHandle` (`self.CameraTimer`)))
        (`self.CameraMoveStart`)))))

(fn `UpdateLockonTarget`
  (params (Target :type "Actor Object Reference"))
  (set `self.ClosedActor` Target))