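; Player lock-on component, apparently meant to aim the camera at an enemy while Space is held, but largely unfinished.
; Tick only validity-checks ClosedEnemy while held and otherwise advances a return timer; ResetCamera, called on release, and SetLockOnCamera are empty.
; CheckScreenDistance, not called here, compares two actors' 2D screen distance to a clamped threshold, relying on GetActorScreenLocation2D, whose viewport-normalised projection nodes are unconnected.
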(event `self.ReceiveTick`
  (params (DeltaSeconds :type "Float (single-precision)"))
  (if (`self.PressLockon`)
    (`/Engine/EditorBlueprintResources/StandardMacros.IsValid` (`self.ClosedEnemy`))
    (elif (not (> (`self.returnSec`) (`self.waitForReturn`)))
      (set `self.returnSec` (+ (`self.returnSec`) (`GameplayStatics.GetWorldDeltaSeconds`))))))

(event `Key|SpaceBar`
  (params (Key :type "Key Structure"))
  (:`Pressed`
    (set `self.PressLockon` true))
  (:`Released`
    (set `self.PressLockon` false)
    (`self.ResetCamera`)))

(fn `CheckScreenDistance`
  (params (A1 :type "Actor Object Reference") (A2 :type "Actor Object Reference") (CheckDistance :type "Float (double-precision)"))
  (returns (bool :type Boolean) (Distance :type "Float (double-precision)"))
  (bind _returnvalue (`KismetMathLibrary.Distance2D` (`self.GetActorScreenLocation2D` A1) (`self.GetActorScreenLocation2D` A2)))
  (`/Engine/EditorBlueprintResources/StandardMacros.IsValid` A1
    (:`Is Valid`
      (`/Engine/EditorBlueprintResources/StandardMacros.IsValid` A2
        (:`Is Valid`
          (return (< _returnvalue (`KismetMathLibrary.FClamp` CheckDistance 0.0 1.212)) _returnvalue))
        (:`Is Not Valid`
          _)))
    (:`Is Not Valid`
      _))
  (return false 0.0))

(fn `ResetCamera`)

(fn `SetLockOnCamera`
  (params (SpringArm :type "SceneComponent Object Reference")))