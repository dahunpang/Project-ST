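; BP_Monster is an AI-controlled monster NPC that exposes attack and retreat events.
; Attack snaps the monster to face the BP_Hunter found in the world, then pulses the Attack flag on its ABP_Monster anim instance for a brief delay.
; TriggerRetreat sets the IsRetreating blackboard key when its controller is a BP_ControllerAI, leaving the retreat behavior itself outside this Blueprint.
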(event `Attack`
  (bind _returnvalue (`GameplayStatics.GetActorOfClass` "/Game/PC/Hunter/BP_Hunter.BP_Hunter_C"))
  (`self.K2_SetActorRotation` (`KismetMathLibrary.FindLookAtRotation` (`self.K2_GetActorLocation`) (`self.K2_GetActorLocation` _returnvalue)))
  (bind _asabp_monster (cast `/Game/NPC/BP/ABP_Monster` (`SkeletalMeshComponent.GetAnimInstance` (`self.Mesh`))))
  (set `/Game/NPC/BP/ABP_Monster.bAttack` true _asabp_monster)
  (`KismetSystemLibrary.Delay` 0.5)
  (set `/Game/NPC/BP/ABP_Monster.bAttack` false _asabp_monster))

(event `TriggerRetreat`
  (cast `/Game/NPC/BP/BP_ControllerAI` (`AIBlueprintHelperLibrary.GetAIController` null))
  (`BlackboardComponent.SetValueAsBool` (`AIBlueprintHelperLibrary.GetBlackboard` null) (`self.IsRetreating`) true))

(fn `UserConstructionScript`)