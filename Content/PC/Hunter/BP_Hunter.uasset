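; Player character for a side-scroller, adding the input mapping and main HUD and handling movement, jump and lock-on, which stops turning.
; Facing-relative directions, attack and jump feed BPCInputBuffer, whose matched commands go to BPCActionComponent to play, save or cancel into actions, gated by notify-state flags.
; The component calls back to play montages, while a state enum blocks movement during actions and is reset on completion from held input and vertical velocity.
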(event `self.ReceiveBeginPlay`
  (bind _asplayer_controller (cast `PlayerController` (`self.GetController` self)))
  (message `EnhancedInputSubsystemInterface.AddMappingContext` (pcsubsystem `EnhancedInputLocalPlayerSubsystem` _asplayer_controller) "/Game/Input/IMC_SideScroller.IMC_SideScroller" 0 (struct))
  (set `self.CurrentState` "NewEnumerator3")
  (bind _returnvalue (`|CreateWidget` "/Game/Ui/Widget/WBP_Main.WBP_Main_C" (`GameplayStatics.GetPlayerController` 0)))
  (`UserWidget.AddToViewport` _returnvalue 0)
  (add `/Game/Blueprints/Component/BPC_ActionComponent.PlayMontage` (`self.BPC_ActionComponent`) (delegate `Play Montage`)))

(event `Play Montage`
  (params (`Action Command` :type "AnimMontage Object Reference") (`Action Id` :type String))
  (bind (_returnvalue_x _returnvalue_y _returnvalue_z) (`KismetMathLibrary.BreakVector` (`CharacterMovementComponent.GetLastUpdateVelocity` (`self.CharacterMovement`))))
  (set `self.CurrentState` "NewEnumerator0")
  (`|PlayMontage` (`self.Mesh`) `Action Command`
    (:`OnCompleted`
      (`|ExecutionSequence`
        (:`then_0`
          (if (`self.IsMovePressing`)
            (set `self.CurrentState` "NewEnumerator5")
            (else
              (set `self.CurrentState` "NewEnumerator3"))))
        (:`then_1`
          (if (> _returnvalue_z 0.1)
            (set `self.CurrentState` "NewEnumerator2")))))))

(event `self.ReceiveTick`
  (params (DeltaSeconds :type "Float (single-precision)")))

(event `EnhancedInput|/Game/Input/IA_LockOn`
  (params (ActionValue :type Boolean) (ElapsedSeconds :type "Float (double-precision)") (TriggeredSeconds :type "Float (double-precision)") (InputAction :type "InputAction Object Reference" :default "/Game/Input/IA_LockOn.IA_LockOn"))
  (:`Started`
    (bind _output_get (set `self.IsLockOn` (not (`self.IsLockOn`))))
    (`KismetSystemLibrary.PrintString` (`KismetStringLibrary.Conv_BoolToString` _output_get))))

(event `EnhancedInput|/Game/Input/IA_Move`
  (params (ActionValue :type "Vector2D Structure") (ElapsedSeconds :type "Float (double-precision)") (TriggeredSeconds :type "Float (double-precision)") (InputAction :type "InputAction Object Reference" :default "/Game/Input/IA_Move.IA_Move"))
  (bind _returnvalue (`KismetMathLibrary.FInterpTo` (`self.InputDirectionSmooth`) ActionValue_X (`GameplayStatics.GetWorldDeltaSeconds`) 20.0))
  (:`Triggered`
    (set `self.IsMovePressing` true)
    (set `self.InputDir` ActionValue_X)
    (set `self.InputDirectionSmooth` _returnvalue)
    (if (`|EnumEquality` (`self.CurrentState`) "NewEnumerator0")
      (bind _input_type (`self.CheckCharacterDirection` (`self.InputDir`)))
      (`/Game/Blueprints/Component/BPC_InputBuffer.AddInput` (`self.BPC_InputBuffer`) (make `/Game/Blueprints/Struct/ST_FInputCommand` _input_type (`KismetSystemLibrary.GetGameTimeInSeconds`)))
      (else
        (set `self.CurrentState` "NewEnumerator5")
        (if (`self.IsLockOn`)
          _
          (elif (< ActionValue_X 0.0)
            (`self.K2_SetActorRotation` (struct :`Yaw` 180.0))
            (else
              (`self.K2_SetActorRotation` (struct)))))
        (`PawnMovementComponent.AddInputVector` (`self.CharacterMovement`) (`KismetMathLibrary.MakeVector` _returnvalue) false)
        (bind _input_type_2 (`self.CheckCharacterDirection` (`self.InputDir`)))
        (`/Game/Blueprints/Component/BPC_InputBuffer.AddInput` (`self.BPC_InputBuffer`) (make `/Game/Blueprints/Struct/ST_FInputCommand` _input_type_2 (`KismetSystemLibrary.GetGameTimeInSeconds`))))))
  (:`Completed`
    (set `self.IsMovePressing` false)
    (if (`|EnumEquality` (`self.CurrentState`) "NewEnumerator0")
      _
      (elif (== ActionValue_X 0.0)
        (set `self.CurrentState` "NewEnumerator3")
        (else
          (set `self.CurrentState` "NewEnumerator5"))))))

(event `EnhancedInput|/Game/Input/IA_Attack`
  (params (ActionValue :type Boolean) (ElapsedSeconds :type "Float (double-precision)") (TriggeredSeconds :type "Float (double-precision)") (InputAction :type "InputAction Object Reference" :default "/Game/Input/IA_Attack.IA_Attack"))
  (bind _bpc_actioncomponent (`self.BPC_ActionComponent`))
  (bind _bpc_actioncomponent_2 (`self.BPC_ActionComponent`))
  (bind _bpc_actioncomponent_3 (`self.BPC_ActionComponent`))
  (:`Started`
    (bind _input_buffer (`/Game/Blueprints/Component/BPC_InputBuffer.AddInput` (`self.BPC_InputBuffer`) (make `/Game/Blueprints/Struct/ST_FInputCommand` "NewEnumerator2")))
    (bind _action_id (`/Game/Blueprints/Component/BPC_InputBuffer.CheckCommandMatch` (`self.BPC_InputBuffer`) _input_buffer))
    (if (not (`/Game/Blueprints/Component/BPC_ActionComponent.ANS_InverseActionCancel` _bpc_actioncomponent))
      (if (`|EnumInequality` (`self.CurrentState`) "NewEnumerator0")
        (`/Game/Blueprints/Component/BPC_ActionComponent.PlayAction` _bpc_actioncomponent _action_id "")
        (elif (`/Game/Blueprints/Component/BPC_ActionComponent.ANS_ActionCancel` (`self.BPC_ActionComponent`))
          (bind _bool (`/Game/Blueprints/Component/BPC_ActionComponent.Check Action Cancel` _bpc_actioncomponent_2 _action_id ""))
          (if _bool
            (`/Game/Blueprints/Component/BPC_ActionComponent.ActionCancel` _bpc_actioncomponent_2 _action_id))))
      (elif (not (`/Game/Blueprints/Component/BPC_ActionComponent.ANS_ActionCancel` _bpc_actioncomponent))
        (`/Game/Blueprints/Component/BPC_ActionComponent.SaveAction` _bpc_actioncomponent _action_id "")
        (else
          (bind _bool_2 (`/Game/Blueprints/Component/BPC_ActionComponent.Check Action Cancel` _bpc_actioncomponent_3 _action_id ""))
          (if _bool_2
            (`/Game/Blueprints/Component/BPC_ActionComponent.ActionCancel` _bpc_actioncomponent_3 _action_id)))))))

(event `EnhancedInput|/Game/Input/IA_Jump`
  (params (ActionValue :type Boolean) (ElapsedSeconds :type "Float (double-precision)") (TriggeredSeconds :type "Float (double-precision)") (InputAction :type "InputAction Object Reference" :default "/Game/Input/IA_Jump.IA_Jump"))
  (:`Started`
    (`self.Jump`)
    (bind _input_buffer (`/Game/Blueprints/Component/BPC_InputBuffer.AddInput` (`self.BPC_InputBuffer`) (make `/Game/Blueprints/Struct/ST_FInputCommand` "NewEnumerator4" (`KismetSystemLibrary.GetGameTimeInSeconds`))))
    (bind _action_id (`/Game/Blueprints/Component/BPC_InputBuffer.CheckCommandMatch` (`self.BPC_InputBuffer`) _input_buffer))
    (`/Game/Blueprints/Component/BPC_ActionComponent.PlayAction` (`self.BPC_ActionComponent`) _action_id "")))

(fn `CheckCharacterDirection`
  (params (InputDir :type "Float (double-precision)"))
  (returns (`Input Type` :type "/Game/PC/Common/Enum_InputType Enum"))
  (if (< (`KismetMathLibrary.Dot_VectorVector` (`self.GetActorForwardVector`) (`KismetMathLibrary.MakeVector` InputDir)) 0.0)
    (return "NewEnumerator1")
    (else
      (return "NewEnumerator0"))))

(fn `UserConstructionScript`)